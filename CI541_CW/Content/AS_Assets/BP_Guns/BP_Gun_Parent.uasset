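; Parent gun Blueprint for a first-person character, attaching the gun mesh to the arms' grip socket and handling hitscan fire and ammo.
; FireBullet line-traces from the owning character's camera, applies damage and physics impulses, plays fire effects, and attaches bullet-hole decals, adding sparks on Robot-tagged actors.
; ReloadGun refills the clip from reserve ammo.
; StartShooting and StopShooting only toggle IsFiring; nothing here calls FireBullet.
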(event `StartShooting`
  (set `self.isFiring` true))

(event `StopShooting`
  (set `self.isFiring` false))

(fn `FireBullet`
  (locals (GunDirection :type "Vector Structure" :default (0.0 0.0 0.0)))
  (bind _bar_ref (`self.Bar_Ref`))
  (bind _asas_bp_first_person_character (cast `/Game/AS_Assets/AS_BP_FirstPersonCharacter` (`self.GetParentActor`)))
  (if (> (`self.AmmoCurrent`) 0)
    (bind _as_firstpersoncamera (`/Game/AS_Assets/AS_BP_FirstPersonCharacter.AS_FirstPersonCamera` _asas_bp_first_person_character))
    (bind _returnvalue (`KismetMathLibrary.GetForwardVector` (`SceneComponent.K2_GetComponentRotation` _as_firstpersoncamera)))
    (set `local.GunDirection` _returnvalue)
    (bind _returnvalue_2 (`SceneComponent.K2_GetComponentLocation` _as_firstpersoncamera))
    (bind _outhit (`KismetSystemLibrary.LineTraceSingle` _returnvalue_2 (+ _returnvalue_2 (* _returnvalue (`self.Distance`))) "TraceTypeQuery1"))
    (`|ExecutionSequence`
      (:`then_0`
        (bind (_bblockinghit _binitialoverlap _time _distance _location _impactpoint _normal _impactnormal _physmat _hitactor _hitcomponent) (`GameplayStatics.BreakHitResult` _outhit))
        (`self.ImpactPhysicsObjects` _bblockinghit _hitcomponent _hitcomponent _location (`local.GunDirection`)))
      (:`then_1`
        (`GameplayStatics.ApplyDamage` _hitactor (`self.Damage`) null null "/Script/Engine.DamageType")
        ;[1 1 1] Play Fire Sound
        (`GameplayStatics.PlaySoundAtLocation` "/Game/MilitaryWeapSilver/Sound/Rifle/Wavs/RifleA_Fire01.RifleA_Fire01" _returnvalue_2 (struct) 1.0 1.0 0.0 null null null null) ; Play firing sound
        (`AnimInstance.Montage_Play` (`SkeletalMeshComponent.GetAnimInstance` (`self.Arms`)) "/Game/FirstPersonArms/Animations/FirstPersonFire_Montage.FirstPersonFire_Montage" 1.0 "MontageLength" 0.0 true)
        (`/Engine/EditorBlueprintResources/StandardMacros.DecrementInt` (`self.AmmoCurrent`)
          (:`  `
            (`GameplayStatics.SpawnEmitterAttached` "/Game/MilitaryWeapSilver/FX/P_AssaultRifle_MuzzleFlash.P_AssaultRifle_MuzzleFlash" _bar_ref "None" (0.0 0.0 0.0) (`SceneComponent.K2_GetComponentRotation` _bar_ref) (1.0 1.0 1.0) "SnapToTargetIncludingScale"))))
      (:`then_2`
        (if _bblockinghit
          (set `self.Decal Material` "/Game/AS_Assets/PNG/MAT_BulletHole.MAT_BulletHole")
          (if (`self.ActorHasTag` _hitactor "Robot")
            (bind _returnvalue_3 (`KismetMathLibrary.MakeRotFromX` _normal))
            (`NiagaraFunctionLibrary.SpawnSystemAtLocation` "/Game/AS_Assets/P_Spark.P_Spark" _location (`KismetMathLibrary.NegateRotator` _returnvalue_3)))
          (bind _returnvalue_4 (`GameplayStatics.SpawnDecalAtLocation` (`self.Decal Material`) (2.0 2.0 2.0) _location _returnvalue_3 10.0))
          (`SceneComponent.K2_AttachToComponent` _returnvalue_4 _hitcomponent "None" "KeepWorld" "KeepWorld" "KeepWorld" true))))))

(fn `ImpactPhysicsObjects`
  (params (IsHitting :type Boolean) (HitComponent :type "SceneComponent Object Reference") (ImpulseObject :type "PrimitiveComponent Object Reference") (Location :type "Vector Structure") (GunDirection :type "Vector Structure"))
  (if IsHitting
    (if (`SceneComponent.IsSimulatingPhysics` HitComponent "None")
      (`PrimitiveComponent.AddImpulseAtLocation` ImpulseObject (* (`local.GunDirection`) (* (`self.Distance`) 10.0)) Location "None"))))

(fn `ReloadGun`
  (locals (BulletDiffrence :type Integer))
  (bind _output_get (set `local.BulletDiffrence` (- (`self.ClipSize`) (`self.AmmoCurrent`))))
  (if (>= (`self.AmmoMax`) _output_get)
    (set `self.AmmoCurrent` (`self.ClipSize`))
    (set `self.AmmoMax` (- (`self.AmmoMax`) (`local.BulletDiffrence`)))
    (else
      (set `self.AmmoCurrent` (+ (`self.AmmoCurrent`) (`self.AmmoMax`)))
      (set `self.AmmoMax` 0))))

(fn `UserConstructionScript`
  (`SceneComponent.K2_AttachToComponent` (`self.Guns`) (`self.Arms`) "GripPoint" "SnapToTarget" "SnapToTarget" "SnapToTarget" true))